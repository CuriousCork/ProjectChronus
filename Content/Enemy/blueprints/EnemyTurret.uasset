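; EnemyTurret is an enemy turret Blueprint that targets the player, fires projectiles and can be destroyed.
; When PawnSensing sees the first-person character, the turret snaps to face it, then spawns an enemy projectile from its Arrow after a delay, which paces the fire.
; Any hit on its Sphere deals fixed damage and prints remaining health; at zero the turret is destroyed with an explosion sound.
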(event OnSeePawn(PawnSensing)
  (params (Pawn :type Pawn%20Object%20Reference))
  ;[0.15 0.15 0.15 0.5] Target Detect And Shoot
  (Utilities|Casting|CastToBP_FirstPersonCharacter Pawn)
  (Transformation|SetActorRotation (Math|Rotator|FindLookatRotation (Transformation|GetActorLocation) (Transformation|GetActorLocation Pawn)))
  (Utilities|FlowControl|Delay 2.5)
  (Game|SpawnActorfromClass "/Game/FirstPerson/Blueprints/BP_FirstPersonProjectileEnemy.BP_FirstPersonProjectileEnemy_C" (Transformation|GetWorldTransform (Variables|Default|GetArrow)) "Undefined" "MultiplyWithRoot" 0 0))

(event OnComponentHit(Sphere)
  (params (HitComponent :type Primitive%20Component%20Object%20Reference) (OtherActor :type Actor%20Object%20Reference) (OtherComp :type Primitive%20Component%20Object%20Reference) (NormalImpulse :type Vector :default "0, 0, 0") (Hit :type Hit%20Result%20Structure%20%28by%20ref%29))
  ;[0.15 0.15 0.15 0.5 41] Damage and Death
  (CallFunction|TakeDamage)
  (Development|PrintString (Utilities|String|ToString(Float) (Variables|Default|GetEnemyHealth))))

(event Custom|takeDamage
  ;[0.15 0.15 0.15 0.5 41] Damage and Death
  (Variables|Default|SetEnemyHealth (- (Variables|Default|GetEnemyHealth) 1e+01))
  (if (<= (Variables|Default|GetEnemyHealth) 0.0)
    (Actor|DestroyActor)
    (Audio|PlaySoundatLocation "/Game/StarterContent/Audio/Explosion01.Explosion01" (Transformation|GetActorLocation) "0, 0, 0" 1.0 1.0 0.0 0 0 0 0)))

(fn ConstructionScript)